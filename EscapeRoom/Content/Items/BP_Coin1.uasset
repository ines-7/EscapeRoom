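; BP_Coin1 is a collectible coin item that the player picks up by interacting with it.
; Its Interact event sets the HasCoin1 flag on the player and passes its item structure to the inventory's OnGetItem call.
; It then plays a cloth movement 2D sound and destroys itself.
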(event `/Game/InventorySystem/InteractInterface.Interact`
  (params (Player :type "/Game/PlayerBlueprint/BP_MyPlayerController Object Reference") (Inventory :type "/Game/WidgetBlueprint/WB_Inventory Object Reference") (`Hit Component` :type "ActorComponent Object Reference"))
  (set `/Game/PlayerBlueprint/BP_MyPlayerController.HasCoin1` true Player)
  (`/Game/WidgetBlueprint/WB_Inventory.OnGetItem` Inventory (`self.Itemstructure`))
  (`GameplayStatics.PlaySound2D` "/Game/Sound/Samples/Cloth_Movement.Cloth_Movement" 1.0 1.0 0.0 null null)
  (`self.K2_DestroyActor`))

(fn `UserConstructionScript`
  (`parent.UserConstructionScript`))