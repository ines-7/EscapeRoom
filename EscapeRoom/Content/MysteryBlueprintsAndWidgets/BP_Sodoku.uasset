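; BP_Sodoku is an interactable, possessable puzzle object that shows the WB_Sodoku widget.
; Interact stores the player, blends the camera to this actor, then possesses it after the blend delay.
; The Interact input then flip-flops between showing the widget with mouse and UI-only input, and removing it, blending back and repossessing the player in game-only input.
; The widget is created once and reused.
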(event `/Game/InventorySystem/InteractInterface.Interact`
  (params (Player :type "/Game/PlayerBlueprint/BP_MyPlayerController Object Reference"))
  (bind _returnvalue (`GameplayStatics.GetPlayerController` 0))
  ;[1 1 1] Start To Interact with Camera Switch
  (bind _output_get (set `self.Player` Player))
  (`PlayerController.SetViewTargetWithBlend` _returnvalue self 0.4 "VTBlend_EaseIn" 0.4 true)
  (`KismetSystemLibrary.Delay` 0.4)
  (`Controller.Possess` _returnvalue self))

(event `InputAction|Interact`
  (params (Key :type "Key Structure"))
  (bind _returnvalue (`GameplayStatics.GetPlayerController` 0))
  ;[1 1 1] Start To Interact with Camera Switch
  (:`Pressed`
    (`/Engine/EditorBlueprintResources/StandardMacros.FlipFlop`
      (:`A`
        (if (not (`self.WidgetExist`))
          (bind _returnvalue_2 (`|CreateWidget` "/Game/MysteryBlueprintsAndWidgets/WB_Sodoku.WB_Sodoku_C")))
        (`UserWidget.AddToViewport` _returnvalue_2 0)
        (set `self.WidgetExist` true)
        (set `PlayerController.bShowMouseCursor` true _returnvalue)
        (`WidgetBlueprintLibrary.SetInputMode_UIOnlyEx` _returnvalue null))
      (:`B`
        (`Widget.RemoveFromParent` _returnvalue_2)
        (`PlayerController.SetViewTargetWithBlend` _returnvalue (stale `/Game/InventorySystem/InteractInterface.Interact` _output_get) 0.4 "VTBlend_EaseOut" 0.4 false)
        (`KismetSystemLibrary.Delay` 0.5)
        (`Controller.Possess` _returnvalue (stale `/Game/InventorySystem/InteractInterface.Interact` _output_get))
        (set `PlayerController.bShowMouseCursor` false _returnvalue)
        (`WidgetBlueprintLibrary.SetInputMode_GameOnly` _returnvalue)))))

(fn `UserConstructionScript`)