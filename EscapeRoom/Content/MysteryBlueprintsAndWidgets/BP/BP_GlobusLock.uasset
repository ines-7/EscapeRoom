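; BP_GlobusLock is an interactable lock actor that opens when the interacting player has the globus key.
; Three chained timelines slide the key mesh in, rotate it, then move the lock ring along Z.
; The key, lock body, ring and cube meshes then start simulating physics, and GlobusSolved receives a SolvedMessage with the player.
; An IsFinished flag, set once the key has turned, blocks later interactions.
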(event `/Game/InventorySystem/InteractInterface.Interact`
  (params (Player :type "/Game/PlayerBlueprint/BP_MyPlayerController Object Reference") (Inventory :type "/Game/WidgetBlueprint/WB_Inventory Object Reference") (`Hit Component` :type "ActorComponent Object Reference"))
  (set `self.Player` Player)
  (if (`self.IsFinished`)
    _
    (elif (`/Game/PlayerBlueprint/BP_MyPlayerController.HasGlobusKey` Player)
      (`SceneComponent.SetVisibility` (`self.SM_Key`) true false)
      (bind (_direction _newtrack_0) (`Timeline|Timeline_0`)
        (:`Update`
          (`SceneComponent.K2_SetRelativeLocation` (`self.SM_Key`) (`KismetMathLibrary.MakeVector` 0.0 _newtrack_0) false false))
        (:`Finished`
          (bind (_direction_2 _newtrack_0_2) (`Timeline|Timeline_1`)
            (:`Update`
              (`SceneComponent.K2_SetRelativeRotation` (`self.SM_Key`) (`KismetMathLibrary.MakeRotator` _newtrack_0_2 0.0 -90.0) false false))
            (:`Finished`
              (set `self.IsFinished` true)
              (bind (_direction_3 _newtrack_0_3) (`Timeline|Timeline_2`)
                (:`Update`
                  (`SceneComponent.K2_SetRelativeLocation` (`self.SM_lock_ring`) (`KismetMathLibrary.MakeVector` 0.0 0.0 _newtrack_0_3) false false))
                (:`Finished`
                  (`PrimitiveComponent.SetSimulatePhysics` (`self.SM_key_lock`) true)
                  (`PrimitiveComponent.SetSimulatePhysics` (`self.SM_Key`) true)
                  (`PrimitiveComponent.SetSimulatePhysics` (`self.Cube`) true)
                  (`PrimitiveComponent.SetSimulatePhysics` (`self.SM_lock_ring`) true)
                  (message `/Game/MysteryBlueprintsAndWidgets/BP/SolvedInterface.Solved` (`KismetSystemLibrary.Conv_InterfaceToObject` (`self.GlobusSolved`)) (`self.Player`)))))))))))

(fn `UserConstructionScript`)