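; BP_Libre is an interactable balance-scale puzzle that takes four coins carried by the player.
; On Interact, while not finished, each newly held coin toggles its mesh's visibility, rotates the balance arms a step and sets that coin's flag.
; Once all four flags are set, it sends SolvedMessage to the linked Belljar through SolvedInterface.
; IsFinished is only read here, never set.
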(event `/Game/InventorySystem/InteractInterface.Interact`
  (params (Player :type "/Game/PlayerBlueprint/BP_MyPlayerController Object Reference") (Inventory :type "/Game/WidgetBlueprint/WB_Inventory Object Reference") (`Hit Component` :type "ActorComponent Object Reference"))
  (bind _belljar (`self.Belljar`))
  (set `self.Player` Player)
  ;[1 1 1] Coin1
  (if (not (`self.IsFinished`))
    (if (`self.Coin1`)
      _
      (elif (`/Game/PlayerBlueprint/BP_MyPlayerController.HasCoin1` (`self.Player`))
        (`SceneComponent.ToggleVisibility` (`self.coins_SM_coin007`) false)
        (`SceneComponent.K2_AddRelativeRotation` (`self.BalanceArmsBase`) (struct :`Pitch` 5.0) false false)
        (set `self.Coin1` true)))
    ;[1 1 1] Coin2
    (if (`self.Coin2`)
      _
      (elif (`/Game/PlayerBlueprint/BP_MyPlayerController.HasCoin2` (`self.Player`))
        (`SceneComponent.ToggleVisibility` (`self.coins_SM_coin008`) false)
        (`SceneComponent.K2_AddRelativeRotation` (`self.BalanceArmsBase`) (struct :`Pitch` 5.0) false false)
        (set `self.Coin2` true)))
    ;[1 1 1] Coin3
    (if (`self.Coin3`)
      _
      (elif (`/Game/PlayerBlueprint/BP_MyPlayerController.HasCoin3` (`self.Player`))
        (`SceneComponent.ToggleVisibility` (`self.coins_SM_coin005`) false)
        (`SceneComponent.K2_AddRelativeRotation` (`self.BalanceArmsBase`) (struct :`Pitch` 5.0) false false)
        (set `self.Coin3` true)))
    ;[1 1 1] Coin4
    (if (`self.Coin4`)
      _
      (elif (`/Game/PlayerBlueprint/BP_MyPlayerController.HasCoin4` (`self.Player`))
        (`SceneComponent.ToggleVisibility` (`self.coins_SM_coin006`) false)
        (`SceneComponent.K2_AddRelativeRotation` (`self.BalanceArmsBase`) (struct :`Pitch` 5.0) false false)
        (set `self.Coin4` true)))
    (if (and (`self.Coin1`) (`self.Coin2`) (`self.Coin3`) (`self.Coin4`))
      (if (`KismetSystemLibrary.DoesImplementInterface` (`KismetSystemLibrary.Conv_InterfaceToObject` _belljar) "/Game/MysteryBlueprintsAndWidgets/BP/SolvedInterface.SolvedInterface_C")
        (message `/Game/MysteryBlueprintsAndWidgets/BP/SolvedInterface.Solved` (`KismetSystemLibrary.Conv_InterfaceToObject` _belljar) (`self.Player`))))))

(fn `UserConstructionScript`)