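; BP_Casket is an interactable puzzle casket that takes three puzzle pieces from the player and opens once all are placed.
; Interact checks each slot in sequence, revealing and sliding in any piece the player holds via its own timeline, then continuing to the next slot.
; When all three are set, a final timeline rolls the Cube component and sets IsFinished, blocking further interaction.
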(event `/Game/InventorySystem/InteractInterface.Interact`
  (params (Player :type "/Game/PlayerBlueprint/BP_MyPlayerController Object Reference") (Inventory :type "/Game/WidgetBlueprint/WB_Inventory Object Reference") (`Hit Component` :type "ActorComponent Object Reference"))
  (set `self.Player` Player)
  (if (`self.isFinished`)
    _
    (elif (`self.HasPuzzle1`)
      (if (`self.HasPuzzle2`) :!label _label
        (if (`self.HasPuzzle3`) :!label _label_2
          ;[1 1 1] Ending
          (if (and (`self.HasPuzzle1`) (`self.HasPuzzle2`) (`self.HasPuzzle3`)) :!label _label_3
            (bind (_direction _newtrack_0) (`Timeline|Timeline_0`)
              (:`Update`
                (`SceneComponent.K2_SetRelativeRotation` (`self.Cube`) (`KismetMathLibrary.MakeRotator` _newtrack_0) false false)
                (set `self.isFinished` true))))
          (else
            ;[1 1 1] PuzzlePiece3
            (if (`/Game/PlayerBlueprint/BP_MyPlayerController.HasPuzzlePiece3` (`self.Player`))
              (`SceneComponent.SetVisibility` (`self.Puzzle3`) true false)
              (bind (_direction_2 _newtrack_0_2) (`Timeline|Timeline_3`)
                (:`Update`
                  (`SceneComponent.K2_SetRelativeLocation` (`self.Puzzle3`) (`KismetMathLibrary.MakeVector` 0.0 _newtrack_0_2) false false))
                (:`Finished`
                  (set `self.HasPuzzle3` true)
                  (goto _label_3)))
              (else
                (goto _label_3)))))
        (else
          ;[1 1 1] Puzzlepiece2
          (if (`/Game/PlayerBlueprint/BP_MyPlayerController.HasPuzzlePiece2` (`self.Player`))
            (`SceneComponent.SetVisibility` (`self.Puzzle2`) true false)
            (bind (_direction_3 _newtrack_0_3) (`Timeline|Timeline_2`)
              (:`Update`
                (`SceneComponent.K2_SetRelativeLocation` (`self.Puzzle2`) (`KismetMathLibrary.MakeVector` 0.0 _newtrack_0_3) false false))
              (:`Finished`
                (set `self.HasPuzzle2` true)
                (goto _label_2)))
            (else
              (goto _label_2)))))
      (else
        ;[1 1 1] Puzzlepiece1
        (if (`/Game/PlayerBlueprint/BP_MyPlayerController.HasPuzzlePiece1` (`self.Player`))
          (`SceneComponent.SetVisibility` (`self.Puzzle1`) true false)
          (bind (_direction_4 _newtrack_0_4) (`Timeline|Timeline_1`)
            (:`Update`
              (`SceneComponent.K2_SetRelativeLocation` (`self.Puzzle1`) (`KismetMathLibrary.MakeVector` 0.0 _newtrack_0_4) false false))
            (:`Finished`
              (set `self.HasPuzzle1` true)
              (goto _label)))
          (else
            (goto _label)))))))

(fn `CheckIfFinished`)

(fn `UserConstructionScript`)