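; BP_Casket is an interactable casket for a three-piece puzzle, apparently where the player places collected pieces.
; Interact stores the player and prints a German "placed" debug message for each piece flag set on that player, without changing any piece state.
; It then calls CheckIfFinished, which tests three unqualified piece flags in nested branches but does nothing when all are true, leaving completion unimplemented.
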(event `/Game/InventorySystem/InteractInterface.Interact`
  (params (Player :type "/Game/PlayerBlueprint/BP_MyPlayerController Object Reference"))
  (set `self.Player` Player)
  (if (`/Game/PlayerBlueprint/BP_MyPlayerController.HasPuzzlePiece1` (`self.Player`))
    (`KismetSystemLibrary.PrintString` "Puzzle Stück 1 Plaziert"))
  (if (`/Game/PlayerBlueprint/BP_MyPlayerController.HasPuzzlePiece2` (`self.Player`))
    (`KismetSystemLibrary.PrintString` "Puzzle Stück 2 Plaziert"))
  (if (`/Game/PlayerBlueprint/BP_MyPlayerController.HasPuzzlePiece3` (`self.Player`))
    (`KismetSystemLibrary.PrintString` "Puzzle Stück 3 Plaziert"))
  (`self.CheckIfFinished`))

(fn `CheckIfFinished`
  (if (`self.hasPuzzlePiece1`)
    (if (`self.hasPuzzlePiece2`)
      (if (`self.hasPuzzlePiece3`)
        _))))

(fn `UserConstructionScript`)