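; BP_bookcase is a moveable bookcase that slides and swings aside when its Solved event is called, apparently as a puzzle reward.
; Solved plays a timeline that lerps the mesh's relative Y from default to a back position, with X and Z fixed.
; A Delay chained to that timeline's update, rather than its finish, then starts a second timeline that lerps the yaw to rotate the bookcase.
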(event `/Game/MysteryBlueprintsAndWidgets/BP/SolvedInterface.Solved`
  (params (Player :type "/Game/PlayerBlueprint/BP_MyPlayerController Object Reference"))
  (bind (_direction _newtrack_0) (`Timeline|Timeline_0` :!via `PlayFromStart`)
    (:`Update`
      (`SceneComponent.K2_SetRelativeLocation` (`self.SM_Moveable_bookcase`) (`KismetMathLibrary.MakeVector` -10.510788 (`KismetMathLibrary.Lerp` (`self.location default`) (`self.movement back`) _newtrack_0) -221.537567) false false)
      (`KismetSystemLibrary.Delay` 3.8)
      (bind (_direction_2 _newtrack_0_2) (`Timeline|Timeline_1`)
        (:`Update`
          (`SceneComponent.K2_SetRelativeRotation` (`self.SM_Moveable_bookcase`) (`KismetMathLibrary.MakeRotator` 0.0 0.0 (`KismetMathLibrary.Lerp` (`self.location/rotation default`) (`self.roation left`) _newtrack_0_2)) false false))))))

(fn `UserConstructionScript`)