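; Possessable chessboard minigame puzzle where the player positions up to three collected chess pieces to solve a Bookshelf puzzle.
; Interact blends the camera, possesses the board, shows WB_Chess and reveals owned pieces using inventory items.
; Input cycles the material-highlighted piece and steps it within per-piece 8x8 grid limits.
; Enter checks three collider overlap flags, then lowers board and pieces, cuts to ChangeCam, notifies Bookshelf and returns control.
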(event `InputAction|Minigame RIGHT`
  (params (Key :type "Key Structure"))
  ;[1 1 1] Figurbewegen
  (:`Pressed`
    (`self.MoveFigur` (0.0 3.8 0.0) 2)))

(event `InputAction|Minigame UP`
  (params (Key :type "Key Structure"))
  ;[1 1 1] Figurbewegen
  (:`Pressed`
    (`self.MoveFigur` (3.8 0.0 0.0))))

(event `self.Collider1.OnComponentBeginOverlap`
  (params (OverlappedComponent :type "PrimitiveComponent Object Reference") (OtherActor :type "Actor Object Reference") (OtherComp :type "PrimitiveComponent Object Reference") (OtherBodyIndex :type Integer) (bFromSweep :type Boolean) (SweepResult :type "HitResult Structure (by ref)"))
  (set `self.Place1` true))

(event `InputAction|Minigame LEFT`
  (params (Key :type "Key Structure"))
  ;[1 1 1] Figurbewegen
  (:`Pressed`
    (`self.MoveFigur` (0.0 -3.8 0.0) 3)))

(event `InputAction|Minigame DOWN`
  (params (Key :type "Key Structure"))
  ;[1 1 1] Figurbewegen
  (:`Pressed`
    (`self.MoveFigur` (-3.8 0.0 0.0) 1)))

(event `self.Collider1.OnComponentEndOverlap`
  (params (OverlappedComponent :type "PrimitiveComponent Object Reference") (OtherActor :type "Actor Object Reference") (OtherComp :type "PrimitiveComponent Object Reference") (OtherBodyIndex :type Integer))
  (set `self.Place1` false))

(event `/Game/InventorySystem/InteractInterface.Interact`
  (params (Player :type "/Game/PlayerBlueprint/BP_MyPlayerController Object Reference") (Inventory :type "/Game/WidgetBlueprint/WB_Inventory Object Reference") (`Hit Component` :type "ActorComponent Object Reference"))
  (bind _returnvalue (`GameplayStatics.GetPlayerController` 0))
  (bind _haschessfigur1 (`/Game/PlayerBlueprint/BP_MyPlayerController.HasChessFigur1` (`self.Player`)))
  (bind _haschessfigur3 (`/Game/PlayerBlueprint/BP_MyPlayerController.HasChessFigur3` (`self.Player`)))
  (bind _haschessfigur2 (`/Game/PlayerBlueprint/BP_MyPlayerController.HasChessFigur2` (`self.Player`)))
  ;[1 1 1] Start To Interact with Camera Switch
  (set `/Game/PlayerBlueprint/BP_MyPlayerController.IsInMinigame` true Player)
  (`/Engine/EditorBlueprintResources/StandardMacros.IsValid` (`self.ChessWB`)
    (:`Is Valid`
      _)
    (:`Is Not Valid`
      (bind _returnvalue_2 (`|CreateWidget` "/Game/MysteryBlueprintsAndWidgets/WB/WB_Chess.WB_Chess_C"))
      (set `self.ChessWB` _returnvalue_2)))
  (if (`self.Isn't Finished`)
    (bind _output_get (set `self.CurrentFigur` (`self.Figur1`)))
    (`MeshComponent.SetScalarParameterValueOnMaterials` _output_get "Density" 1.0)
    (`MeshComponent.SetScalarParameterValueOnMaterials` _output_get "isHighlighted" 1.0))
  (bind _output_get_2 (set `self.Player` Player))
  (`PlayerController.SetViewTargetWithBlend` _returnvalue self 0.4 "VTBlend_Cubic" 0.4 true)
  (`KismetSystemLibrary.Delay` 0.6)
  (`Controller.Possess` _returnvalue self)
  (`UserWidget.AddToViewport` (`self.ChessWB`) 0)
  (if _haschessfigur1
    (`/Game/WidgetBlueprint/WB_Inventory.OnUseItem` Inventory 11)
    (`KismetSystemLibrary.Delay` 0.2)
    (`SceneComponent.SetVisibility` (`self.Figur1`) _haschessfigur1 false)
    (set `self.PlayerHasFigur1` _haschessfigur1))
  (if _haschessfigur2
    (`/Game/WidgetBlueprint/WB_Inventory.OnUseItem` Inventory 12)
    (`SceneComponent.SetVisibility` (`self.Figur2`) _haschessfigur2 false)
    (set `self.PlayerHasFigur2` _haschessfigur2))
  (if _haschessfigur3
    (`/Game/WidgetBlueprint/WB_Inventory.OnUseItem` Inventory 13)
    (`SceneComponent.SetVisibility` (`self.Figur3`) _haschessfigur3 false)
    (set `self.PlayerHasFigur3` _haschessfigur3)))

(event `self.Collider2.OnComponentBeginOverlap`
  (params (OverlappedComponent :type "PrimitiveComponent Object Reference") (OtherActor :type "Actor Object Reference") (OtherComp :type "PrimitiveComponent Object Reference") (OtherBodyIndex :type Integer) (bFromSweep :type Boolean) (SweepResult :type "HitResult Structure (by ref)"))
  (set `self.Place2` true))

(event `InputAction|Minigame Next`
  (params (Key :type "Key Structure"))
  (:`Pressed`
    (`self.SwitchFigur`)))

(event `self.Collider2.OnComponentEndOverlap`
  (params (OverlappedComponent :type "PrimitiveComponent Object Reference") (OtherActor :type "Actor Object Reference") (OtherComp :type "PrimitiveComponent Object Reference") (OtherBodyIndex :type Integer))
  (set `self.Place2` false))

(event `self.Collider3.OnComponentBeginOverlap`
  (params (OverlappedComponent :type "PrimitiveComponent Object Reference") (OtherActor :type "Actor Object Reference") (OtherComp :type "PrimitiveComponent Object Reference") (OtherBodyIndex :type Integer) (bFromSweep :type Boolean) (SweepResult :type "HitResult Structure (by ref)"))
  (set `self.Place3` true))

(event `InputAction|Minigame ENTER`
  (params (Key :type "Key Structure"))
  (bind _returnvalue (`GameplayStatics.GetPlayerController` 0))
  (bind _player (`self.Player`))
  (:`Pressed`
    (`self.CheckIfEnd`)
    (if (not (`self.Isn't Finished`))
      (`Timeline|Timeline_0`
        (:`Update`
          (`SceneComponent.K2_AddRelativeLocation` (`self.SM_Chessboard_SM_C2`) (0.0 0.0 -0.003) false false)
          (`SceneComponent.K2_AddRelativeLocation` (`self.SM_Chessboard_SM_C4`) (0.0 0.0 -0.003) false false)
          (`SceneComponent.K2_AddRelativeLocation` (`self.SM_Chessboard_SM_D6`) (0.0 0.0 -0.003) false false)
          (`SceneComponent.K2_AddRelativeLocation` (`self.Figur1`) (0.0 0.0 -0.003) false false)
          (`SceneComponent.K2_AddRelativeLocation` (`self.Figur2`) (0.0 0.0 -0.003) false false)
          (`SceneComponent.K2_AddRelativeLocation` (`self.Figur3`) (0.0 0.0 -0.003) false false))
        (:`Finished`
          (`Widget.RemoveFromParent` (`self.ChessWB`))
          (`PlayerController.SetViewTargetWithBlend` _returnvalue (`self.Change Cam`) 2.0 "VTBlend_Linear" 0.0 false)
          (`KismetSystemLibrary.Delay` 3.0)
          (message `/Game/MysteryBlueprintsAndWidgets/BP/SolvedInterface.Solved` (`self.Bookshelf`) null)
          (`KismetSystemLibrary.Delay` 6.5)
          (`PlayerController.SetViewTargetWithBlend` _returnvalue _player 1.0 "VTBlend_Cubic" 0.4 false)
          (`KismetSystemLibrary.Delay` 0.6)
          (`Controller.Possess` _returnvalue _player)
          (set `/Game/PlayerBlueprint/BP_MyPlayerController.IsInMinigame` false (`self.Player`))
          (`Widget.RemoveFromParent` (`self.ChessWB`))
          (`MeshComponent.SetScalarParameterValueOnMaterials` (`self.CurrentFigur`) "isHighlighted" 0.0))))))

(event `InputAction|Interact`
  (params (Key :type "Key Structure"))
  (bind _returnvalue (`GameplayStatics.GetPlayerController` 0))
  ;[1 1 1] Start To Interact with Camera Switch
  (:`Pressed`
    (`PlayerController.SetViewTargetWithBlend` _returnvalue (stale `/Game/InventorySystem/InteractInterface.Interact` _output_get_2) 0.4 "VTBlend_Cubic" 0.4 false)
    (`KismetSystemLibrary.Delay` 0.6)
    (`Controller.Possess` _returnvalue (stale `/Game/InventorySystem/InteractInterface.Interact` _output_get_2))
    (set `/Game/PlayerBlueprint/BP_MyPlayerController.IsInMinigame` false (`self.Player`))
    (`Widget.RemoveFromParent` (`self.ChessWB`))
    (`MeshComponent.SetScalarParameterValueOnMaterials` (`self.CurrentFigur`) "isHighlighted" 0.0)))

(event `self.Collider3.OnComponentEndOverlap`
  (params (OverlappedComponent :type "PrimitiveComponent Object Reference") (OtherActor :type "Actor Object Reference") (OtherComp :type "PrimitiveComponent Object Reference") (OtherBodyIndex :type Integer))
  (set `self.Place3` false))

(fn `CheckIfEnd`
  (if (`self.Isn't Finished`)
    (if (`self.Place1`)
      (if (`self.Place2`)
        (if (`self.Place3`)
          (`KismetSystemLibrary.PrintString` "Rätsel Fertig")
          (set `self.Isn't Finished` false)
          (`MeshComponent.SetScalarParameterValueOnMaterials` (`self.CurrentFigur`) "isHighlighted" 0.0))))))

(fn `MoveFigur`
  (params (`Delta Location` :type "Vector Structure") (Direction :type Integer))
  (bind _figur1counterhorizontal (`self.Figur1CounterHorizontal`))
  (bind _figur2counterhorizontal (`self.Figur2CounterHorizontal`))
  (bind _figur2countervertical (`self.Figur2CounterVertical`))
  (bind _figur3counterhorizontal (`self.Figur3CounterHorizontal`))
  (bind _figur3countervertical (`self.Figur3CounterVertical`))
  (bind _figur1countervertical (`self.Figur1CounterVertical`))
  (bind _figur1counterhorizontal_2 (`self.Figur1CounterHorizontal`))
  (if (`self.Isn't Finished`)
    (switch `int` (`self.Figurcounter`)
      (:`0`
        (if (`self.PlayerHasFigur1`)
          (switch `int` Direction
            (:`Default`
              (`SceneComponent.K2_AddRelativeLocation` (`self.CurrentFigur`) `Delta Location` false false :!label _label))
            (:`0`
              (if (> _figur1counterhorizontal_2 0)
                (`/Engine/EditorBlueprintResources/StandardMacros.DecrementInt` _figur1counterhorizontal_2
                  (:`  `
                    (goto _label)))))
            (:`1`
              (if (< _figur1counterhorizontal 7)
                (`/Engine/EditorBlueprintResources/StandardMacros.IncrementInt` _figur1counterhorizontal
                  (:`  `
                    (goto _label)))))
            (:`2`
              (if (< _figur1countervertical 7)
                (`/Engine/EditorBlueprintResources/StandardMacros.IncrementInt` _figur1countervertical
                  (:`  `
                    (goto _label)))))
            (:`3`
              (if (> _figur1countervertical 0)
                (`/Engine/EditorBlueprintResources/StandardMacros.DecrementInt` _figur1countervertical
                  (:`  `
                    (goto _label))))))))
      (:`1`
        (if (`self.PlayerHasFigur2`)
          (switch `int` Direction
            (:`0`
              (if (> _figur2counterhorizontal 0)
                (`/Engine/EditorBlueprintResources/StandardMacros.DecrementInt` _figur2counterhorizontal
                  (:`  `
                    (goto _label)))))
            (:`1`
              (if (< _figur2counterhorizontal 7)
                (`/Engine/EditorBlueprintResources/StandardMacros.IncrementInt` _figur2counterhorizontal
                  (:`  `
                    (goto _label)))))
            (:`2`
              (if (< _figur2countervertical 7)
                (`/Engine/EditorBlueprintResources/StandardMacros.IncrementInt` _figur2countervertical
                  (:`  `
                    (goto _label)))))
            (:`3`
              (if (> _figur2countervertical 0)
                (`/Engine/EditorBlueprintResources/StandardMacros.DecrementInt` _figur2countervertical
                  (:`  `
                    (goto _label))))))))
      (:`2`
        (if (`self.PlayerHasFigur3`)
          (switch `int` Direction
            (:`0`
              (if (> _figur3counterhorizontal 0)
                (`/Engine/EditorBlueprintResources/StandardMacros.DecrementInt` _figur3counterhorizontal
                  (:`  `
                    (goto _label)))))
            (:`1`
              (if (< _figur3counterhorizontal 7)
                (`/Engine/EditorBlueprintResources/StandardMacros.IncrementInt` _figur3counterhorizontal
                  (:`  `
                    (goto _label)))))
            (:`2`
              (if (< _figur3countervertical 7)
                (`/Engine/EditorBlueprintResources/StandardMacros.IncrementInt` _figur3countervertical
                  (:`  `
                    (goto _label)))))
            (:`3`
              (if (> _figur3countervertical 0)
                (`/Engine/EditorBlueprintResources/StandardMacros.DecrementInt` _figur3countervertical
                  (:`  `
                    (goto _label)))))))))))

(fn `SwitchFigur`
  (if (`self.Isn't Finished`)
    (`MeshComponent.SetScalarParameterValueOnMaterials` (`self.CurrentFigur`) "isHighlighted" 0.0)
    (bind _result (`/Engine/EditorBlueprintResources/StandardMacros.IncrementInt` (`self.Figurcounter`))
      (:`  `
        (switch `int` _result
          (:`0`
            (bind _output_get (set `self.CurrentFigur` (`self.Figur1`) :!label _label))
            (`MeshComponent.SetScalarParameterValueOnMaterials` _output_get "isHighlighted" 1.0)
            (`MeshComponent.SetScalarParameterValueOnMaterials` _output_get "Density" 1.5))
          (:`1`
            (bind _output_get_2 (set `self.CurrentFigur` (`self.Figur2`)))
            (`MeshComponent.SetScalarParameterValueOnMaterials` _output_get_2 "isHighlighted" 1.0)
            (`MeshComponent.SetScalarParameterValueOnMaterials` _output_get_2 "Density" 1.5))
          (:`2`
            (bind _output_get_3 (set `self.CurrentFigur` (`self.Figur3`)))
            (`MeshComponent.SetScalarParameterValueOnMaterials` _output_get_3 "isHighlighted" 1.0)
            (`MeshComponent.SetScalarParameterValueOnMaterials` _output_get_3 "Density" 1.5))
          (:`3`
            (set `self.Figurcounter` 0)
            (goto _label)))))))

(fn `UserConstructionScript`)