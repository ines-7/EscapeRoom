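; Possessable chessboard puzzle minigame where the player moves up to three chess figures onto target places.
; Interact blends the camera to the board, possesses it, shows the WB_Chess widget and reveals figures the player holds; interacting again returns control.
; Inputs nudge the current figure in fixed steps or cycle selection, highlighted through a material parameter.
; Three colliders set occupancy flags without checking what overlaps; Enter marks the puzzle finished when all are set.
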(event `InputAction|Minigame UP`
  (params (Key :type "Key Structure"))
  ;[1 1 1] Figurbewegen
  (:`Pressed`
    (if (`self.PlayerHasFigur1`)
      (if (`self.Isn't Finished`)
        (`SceneComponent.K2_SetWorldLocation` (`self.CurrentFigur`) (+ (`SceneComponent.K2_GetComponentLocation` (`self.CurrentFigur`)) (3.8 0.0 0.0)) false false)))))

(event `InputAction|Minigame RIGHT`
  (params (Key :type "Key Structure"))
  ;[1 1 1] Figurbewegen
  (:`Pressed`
    (if (`self.PlayerHasFigur1`)
      (if (`self.Isn't Finished`)
        (`SceneComponent.K2_SetWorldLocation` (`self.CurrentFigur`) (+ (`SceneComponent.K2_GetComponentLocation` (`self.CurrentFigur`)) (0.0 3.8 0.0)) false false)))))

(event `/Game/InventorySystem/InteractInterface.Interact`
  (params (Player :type "/Game/PlayerBlueprint/BP_MyPlayerController Object Reference"))
  (bind _returnvalue (`GameplayStatics.GetPlayerController` 0))
  (bind _haschessfigur1 (`/Game/PlayerBlueprint/BP_MyPlayerController.HasChessFigur1` (`self.Player`)))
  (bind _haschessfigur3 (`/Game/PlayerBlueprint/BP_MyPlayerController.HasChessFigur3` (`self.Player`)))
  (bind _haschessfigur2 (`/Game/PlayerBlueprint/BP_MyPlayerController.HasChessFigur2` (`self.Player`)))
  ;[1 1 1] Start To Interact with Camera Switch
  (`/Engine/EditorBlueprintResources/StandardMacros.IsValid` (`self.ChessWB`)
    (:`Is Valid`
      _)
    (:`Is Not Valid`
      (bind _returnvalue_2 (`|CreateWidget` "/Game/MysteryBlueprintsAndWidgets/WB_Chess.WB_Chess_C"))
      (set `self.ChessWB` _returnvalue_2)))
  (bind _output_get (set `self.CurrentFigur` (`self.Figur1`)))
  (`MeshComponent.SetScalarParameterValueOnMaterials` _output_get "isHighlighted" 1.0)
  (bind _output_get_2 (set `self.Player` Player))
  (`PlayerController.SetViewTargetWithBlend` _returnvalue self 0.4 "VTBlend_Cubic" 0.4 true)
  (`KismetSystemLibrary.Delay` 0.6)
  (`Controller.Possess` _returnvalue self)
  (`UserWidget.AddToViewport` (`self.ChessWB`) 0)
  (if _haschessfigur1
    (`KismetSystemLibrary.Delay` 0.2)
    (`SceneComponent.SetVisibility` (`self.Figur1`) _haschessfigur1 false)
    (set `self.PlayerHasFigur1` _haschessfigur1)
    (if _haschessfigur2
      (`SceneComponent.SetVisibility` (`self.Figur2`) _haschessfigur2 false)
      (set `self.PlayerHasFigur2` _haschessfigur2)
      (if _haschessfigur3
        (`SceneComponent.SetVisibility` (`self.Figur3`) _haschessfigur3 false)
        (set `self.PlayerHasFigur3` _haschessfigur3)))))

(event `InputAction|Minigame Next`
  (params (Key :type "Key Structure"))
  (bind _figur1 (`self.Figur1`))
  (bind _figur2 (`self.Figur2`))
  ;[1 1 1] Figurswitch
  (:`Pressed`
    (bind _result (`/Engine/EditorBlueprintResources/StandardMacros.IncrementInt` (`self.Figurcounter`))
      (:`  `
        (`MeshComponent.SetScalarParameterValueOnMaterials` (`self.CurrentFigur`) "isHighlighted " 0.0)
        (switch `int` _result
          (:`0`
            (bind _output_get (set `self.CurrentFigur` _figur1 :!label _label))
            (`MeshComponent.SetScalarParameterValueOnMaterials` _output_get "isHighlighted" 1.0)
            (`MeshComponent.SetScalarParameterValueOnMaterials` _figur2 "isHighlighted " 0.0)
            (`MeshComponent.SetScalarParameterValueOnMaterials` (`self.Figur3`) "isHighlighted " 0.0))
          (:`1`
            (bind _output_get_2 (set `self.CurrentFigur` _figur2))
            (`MeshComponent.SetScalarParameterValueOnMaterials` _output_get_2 "isHighlighted" 1.0)
            (`MeshComponent.SetScalarParameterValueOnMaterials` _figur1 "isHighlighted " 0.0)
            (`MeshComponent.SetScalarParameterValueOnMaterials` (stale _output_get_3) "isHighlighted " 0.0))
          (:`2`
            (bind _output_get_3 (set `self.CurrentFigur` (`self.Figur3`)))
            (`MeshComponent.SetScalarParameterValueOnMaterials` _output_get_3 "isHighlighted" 1.0)
            (`MeshComponent.SetScalarParameterValueOnMaterials` _figur1 "isHighlighted " 0.0)
            (`MeshComponent.SetScalarParameterValueOnMaterials` _figur2 "isHighlighted " 0.0))
          (:`3`
            (set `self.Figurcounter` 0)
            (goto _label)))))))

(event `InputAction|Minigame LEFT`
  (params (Key :type "Key Structure"))
  ;[1 1 1] Figurbewegen
  (:`Pressed`
    (if (`self.PlayerHasFigur1`)
      (if (`self.Isn't Finished`)
        (`SceneComponent.K2_SetWorldLocation` (`self.CurrentFigur`) (+ (`SceneComponent.K2_GetComponentLocation` (`self.CurrentFigur`)) (0.0 -3.8 0.0)) false false)))))

(event `InputAction|Minigame DOWN`
  (params (Key :type "Key Structure"))
  ;[1 1 1] Figurbewegen
  (:`Pressed`
    (if (`self.PlayerHasFigur1`)
      (if (`self.Isn't Finished`)
        (`SceneComponent.K2_SetWorldLocation` (`self.CurrentFigur`) (+ (`SceneComponent.K2_GetComponentLocation` (`self.CurrentFigur`)) (-3.8 0.0 0.0)) false false)))))

(event `InputAction|Interact`
  (params (Key :type "Key Structure"))
  (bind _returnvalue (`GameplayStatics.GetPlayerController` 0))
  ;[1 1 1] Start To Interact with Camera Switch
  (:`Pressed`
    (`PlayerController.SetViewTargetWithBlend` _returnvalue (stale `/Game/InventorySystem/InteractInterface.Interact` _output_get_2) 0.4 "VTBlend_Cubic" 0.4 false)
    (`KismetSystemLibrary.Delay` 0.6)
    (`Controller.Possess` _returnvalue (stale `/Game/InventorySystem/InteractInterface.Interact` _output_get_2))
    (set `/Game/PlayerBlueprint/BP_MyPlayerController.IsInMinigame` false (`self.Player`))
    (`Widget.RemoveFromParent` (`self.ChessWB`))
    (`MeshComponent.SetScalarParameterValueOnMaterials` (`self.CurrentFigur`) "isHighlighted " 0.0)))

(event `self.Collider1.OnComponentBeginOverlap`
  (params (OverlappedComponent :type "PrimitiveComponent Object Reference") (OtherActor :type "Actor Object Reference") (OtherComp :type "PrimitiveComponent Object Reference") (OtherBodyIndex :type Integer) (bFromSweep :type Boolean) (SweepResult :type "HitResult Structure (by ref)"))
  (set `self.Place1` true))

(event `self.Collider1.OnComponentEndOverlap`
  (params (OverlappedComponent :type "PrimitiveComponent Object Reference") (OtherActor :type "Actor Object Reference") (OtherComp :type "PrimitiveComponent Object Reference") (OtherBodyIndex :type Integer))
  (set `self.Place1` false))

(event `self.Collider2.OnComponentBeginOverlap`
  (params (OverlappedComponent :type "PrimitiveComponent Object Reference") (OtherActor :type "Actor Object Reference") (OtherComp :type "PrimitiveComponent Object Reference") (OtherBodyIndex :type Integer) (bFromSweep :type Boolean) (SweepResult :type "HitResult Structure (by ref)"))
  (set `self.Place2` true))

(event `InputAction|Minigame ENTER`
  (params (Key :type "Key Structure"))
  ;[1 1 1] Figur
  (:`Pressed`
    (if (`self.Isn't Finished`)
      (if (`self.Place1`)
        (if (`self.Place2`)
          (if (`self.Place3`)
            (`KismetSystemLibrary.PrintString` "Rätsel Fertig")
            (set `self.Isn't Finished` false)))))))

(event `self.Collider2.OnComponentEndOverlap`
  (params (OverlappedComponent :type "PrimitiveComponent Object Reference") (OtherActor :type "Actor Object Reference") (OtherComp :type "PrimitiveComponent Object Reference") (OtherBodyIndex :type Integer))
  (set `self.Place2` false))

(event `self.Collider3.OnComponentBeginOverlap`
  (params (OverlappedComponent :type "PrimitiveComponent Object Reference") (OtherActor :type "Actor Object Reference") (OtherComp :type "PrimitiveComponent Object Reference") (OtherBodyIndex :type Integer) (bFromSweep :type Boolean) (SweepResult :type "HitResult Structure (by ref)"))
  (set `self.Place3` true))

(event `self.Collider3.OnComponentEndOverlap`
  (params (OverlappedComponent :type "PrimitiveComponent Object Reference") (OtherActor :type "Actor Object Reference") (OtherComp :type "PrimitiveComponent Object Reference") (OtherBodyIndex :type Integer))
  (set `self.Place3` false))

(fn `UserConstructionScript`)